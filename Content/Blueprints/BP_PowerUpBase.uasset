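; Base power-up pill for an Arkanoid-style game that falls toward the player and grants a power-up when caught.
; On BeginPlay it launches the pill along negative X at FallSpeed and picks its material by indexing Materials with the Powerup value.
; Only overlap with BP_ArkanoidPlayerBase passes Powerup to AddPowerup and destroys the pill.
; DoPowerup is a stub that returns false.
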(event `self.ReceiveBeginPlay`
  ;[1 1 1] Move the Pill down the X Axis
  (`PrimitiveComponent.AddImpulse` (`self.PowerPill`) (`KismetMathLibrary.MakeVector` (* -1.0 (`self.Fall Speed`))) "None" true)
  (`PrimitiveComponent.SetMaterial` (`self.PowerPill`) 0 (`|GetArrayItem` (`self.Materials`) (`KismetMathLibrary.Conv_ByteToInt` (`self.Powerup`)))))

(event `self.ReceiveActorBeginOverlap`
  (params (OtherActor :type "Actor Object Reference"))
  ;[1 1 1] Only Let Player Base Destroy on Overlap!
  (bind _asbp_arkanoid_player_base (cast `/Game/Blueprints/BP_ArkanoidPlayerBase` OtherActor))
  (`/Game/Blueprints/BP_ArkanoidPlayerBase.Add Powerup` _asbp_arkanoid_player_base (`self.Powerup`))
  (`self.K2_DestroyActor`))

(fn `DoPowerup`
  (params (Player :type "/Game/Blueprints/BP_ArkanoidPlayerBase Object Reference"))
  (returns (Result :type Boolean))
  (return false))

(fn `UserConstructionScript`)