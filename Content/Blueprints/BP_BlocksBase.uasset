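; BP_BlocksBase is the breakable block for an Arkanoid-style game, damaged by ball or projectile hits and overlaps.
; On BeginPlay it registers with the game mode, adds toughness every seven levels and creates a dynamic material.
; Surviving hits play an Alpha timeline on that material, with sound only for non-overlap hits.
; Breaking awards points, updates the remaining count, sometimes spawns a random powerup via a randomized counter modulo, then destroys itself.
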(event `self.ReceiveBeginPlay`
  (bind _block (`self.Block`))
  ;[1 1 1] Event Begin Play
  (bind _asbp_arkanoid_game (cast `/Game/Blueprints/BP_ArkanoidGame` (`GameplayStatics.GetGameMode`)))
  (bind _output_get (set `self.Game Mode` _asbp_arkanoid_game))
  (`/Game/Blueprints/BP_ArkanoidGame.Add to Remaning Blocks` _output_get)
  (bind _asbp_game_instance (cast `/Game/Blueprints/BP_GameInstance` (`GameplayStatics.GetGameInstance`)))
  (set `self.HitsToBreak` (+ (`self.HitsToBreak`) (/ (- (`/Game/Blueprints/BP_GameInstance.CurrentLevel` _asbp_game_instance) 1) 7)))
  (bind _returnvalue (`PrimitiveComponent.CreateDynamicMaterialInstance` _block 0 (`PrimitiveComponent.GetMaterial` _block 0) "None"))
  (set `self.Dynamic Material` _returnvalue))

(event `self.Block.OnComponentBeginOverlap`
  (params (OverlappedComponent :type "PrimitiveComponent Object Reference") (OtherActor :type "Actor Object Reference") (OtherComp :type "PrimitiveComponent Object Reference") (OtherBodyIndex :type Integer) (bFromSweep :type Boolean) (SweepResult :type "HitResult Structure (by ref)"))
  ;[0.2159 0.006049 0.005605] Handle Damage by Hit (Ball) or Overlap (Projectiles)
  (`self.Handle Damage` OtherActor true))

(event `self.Block.OnComponentHit`
  (params (HitComponent :type "PrimitiveComponent Object Reference") (OtherActor :type "Actor Object Reference") (OtherComp :type "PrimitiveComponent Object Reference") (NormalImpulse :type "Vector Structure") (Hit :type "HitResult Structure (by ref)"))
  ;[0.2159 0.006049 0.005605] Handle Damage by Hit (Ball) or Overlap (Projectiles)
  (`self.Handle Damage` OtherActor))

(event `Handle Damage`
  (params (`Hit Actor` :type "Actor Object Reference") (`Is Overlap` :type Boolean))
  (bind (_returnvalue_location _returnvalue_rotation) (`KismetMathLibrary.BreakTransform` (`self.GetTransform`)))
  (bind _game_mode (`self.Game Mode`))
  ;[1 1 1] Handle Damage
  (if (or (`.bSuccess` (cast `/Game/Blueprints/BP_TheBall` `Hit Actor` :!pure true)) (`.bSuccess` (cast `/Game/Blueprints/BP_Projectile` `Hit Actor` :!pure true)))
    (bind _result (`/Engine/EditorBlueprintResources/StandardMacros.DecrementInt` (`self.HitsToBreak`))
      (:`  `
        (if (<= _result 0)
          ;;[1 1 1] Add points Based on Block Points Variable
          (`/Game/Blueprints/BP_ArkanoidGame.Add Points` _game_mode (`self.Block Points`))
          (`/Game/Blueprints/BP_ArkanoidGame.Subtract from Remaining Blocks` _game_mode)
          (if (`self.Should Spawn Powerup`)
            (`|SpawnActorFromClass` "/Game/Blueprints/BP_PowerUpBase.BP_PowerUpBase_C" (`KismetMathLibrary.MakeTransform` _returnvalue_location _returnvalue_rotation (1.2 1.2 1.2)) "AlwaysSpawn" "OverrideRootScale" null (cast `/Game/Blueprints/E_Powerups` (`KismetMathLibrary.Conv_IntToByte` (`KismetMathLibrary.RandomIntegerInRange` 0 (- (enumcount `/Game/Blueprints/E_Powerups`) 1)))) null))
          (`GameplayStatics.PlaySound2D` "/Game/Sounds/Cue/Hit_Block_Cue.Hit_Block_Cue" 1.0 1.0 0.0 null null)
          (`self.K2_DestroyActor`)
          (elif `Is Overlap`
            (bind (_direction _alpha) (`Timeline|Alpha` :!via `PlayFromStart` :!label _label)
              (:`Update`
                (`MaterialInstanceDynamic.SetScalarParameterValue` (`self.Dynamic Material`) "Alpha" _alpha)))
            (else
              (`GameplayStatics.PlaySound2D` (`self.SoundEffect`) 1.0 1.0 0.0 null null)
              (goto _label :!via `PlayFromStart`))))))))

(fn `Should Spawn Powerup`
  (returns (Result :type Boolean))
  (return (== (mod (`/Game/Blueprints/BP_ArkanoidGame.Powerup Block Counter` (`self.Game Mode`)) (`KismetMathLibrary.RandomIntegerInRange` 3 7)) 0)))

(fn `UserConstructionScript`)