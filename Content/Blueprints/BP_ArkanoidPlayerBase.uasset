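; Player paddle base for an Arkanoid game, handling physics movement, ball catching and launching, laser fire, lives, pausing and warp exit.
; Tracks active balls, dying when the last is removed, then respawning through material-parameter timelines or showing game over.
; Stores powerups as a bitmask; incompatible pickups clear existing ones before applying effects to paddle, balls, lives or side exit.
; Tick eases paddle scale and clamps it within level bounds; number keys trigger debug powerups.
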(event `InputAction|PauseGame` :paused true
  (params (Key :type "Key Structure"))
  (bind _player_controller (`self.Player Controller`))
  (bind _wbp_pausemenu (`/Game/Widgets/WBP_ArkanoidHUDWidget.WBP_PauseMenu` (`/Game/Blueprints/BP_ArkanoidGame.HUDWidget` (`self.Game Mode`))))
  ;[1 1 1] Pause Function
  (:`Pressed`
    (if (`GameplayStatics.IsGamePaused`)
      (`/Game/Blueprints/BP_ArkanoidGame.UnpauseEvent` (`self.Game Mode`))
      (else
        (`GameplayStatics.SetGamePaused` true)
        (`Widget.SetVisibility` _wbp_pausemenu "Visible")
        (set `PlayerController.bShowMouseCursor` true _player_controller)
        (`WidgetBlueprintLibrary.SetInputMode_GameAndUIEx` _player_controller (`/Game/Widgets/WBP_PauseMenu.Unpause_Button` _wbp_pausemenu))))))

(event `self.ReceiveTick`
  (params (DeltaSeconds :type "Float (single-precision)"))
  (bind (_returnvalue_x _returnvalue_y _returnvalue_z) (`KismetMathLibrary.BreakVector` (`self.K2_GetActorLocation`)))
  (bind (_bounds_x _bounds_y) (`KismetMathLibrary.BreakVector` (`self.Bounds`)))
  (bind _returnvalue (- (`self.Level Bounds`) (- (+ (.y (`.BoxExtent` (`self.GetActorBounds` false))) -90.0) _bounds_y)))
  ;[1 1 1] Tick -
  (if (`self.Warp Out`)
    (`PrimitiveComponent.AddForce` (`self.paddle`) (0.0 20000.0 0.0) "None" true)
    (else
      (`self.SetActorScale3D` (`KismetMathLibrary.VInterpTo_Constant` (`self.GetActorScale3D`) (`self.Target Scale`) DeltaSeconds 3.0))
      (`self.K2_SetActorLocation` (`KismetMathLibrary.MakeVector` _returnvalue_x (`KismetMathLibrary.FClamp` _returnvalue_y (* _returnvalue -0.95) _returnvalue) _returnvalue_z)))))

(event `self.ReceiveHit`
  (params (MyComp :type "PrimitiveComponent Object Reference") (Other :type "Actor Object Reference") (OtherComp :type "PrimitiveComponent Object Reference") (bSelfMoved :type Boolean) (HitLocation :type "Vector Structure") (HitNormal :type "Vector Structure") (NormalImpulse :type "Vector Structure") (Hit :type "HitResult Structure (by ref)"))
  (bind (_returnvalue_x _returnvalue_y) (`KismetMathLibrary.BreakVector` (`KismetMathLibrary.InverseTransformLocation` (`self.GetTransform`) (`.ImpactPoint` (`GameplayStatics.BreakHitResult` Hit)))))
  ;[1 1 1] On Hit Event - sound, check for catch powerup, and some needed calculations
  (bind _asbp_the_ball (cast `/Game/Blueprints/BP_TheBall` Other))
  (`GameplayStatics.PlaySound2D` "/Game/Sounds/Cue/Hit_Paddle_Cue.Hit_Paddle_Cue" 1.0 1.0 0.0 null null)
  (if (`self.Has Powerup` "NewEnumerator0")
    (`self.Put Ball In Paddle` _asbp_the_ball _returnvalue_y)
    ;[1 1 1] Delay then Launch the ball - for catch fairness
    (`KismetSystemLibrary.Delay` 3.0)
    (`self.Launch Ball In Paddle`)))

(event `self.ReceiveBeginPlay`
  ;[0.2159 0.006049 0.005605] EVENT BEGIN PLAY - Attach The Ball To This Player Base
  (bind _asbp_game_instance (cast `/Game/Blueprints/BP_GameInstance` (`GameplayStatics.GetGameInstance`)))
  (set `self.GameInstance` _asbp_game_instance)
  (bind _asbp_arkanoid_game (cast `/Game/Blueprints/BP_ArkanoidGame` (`GameplayStatics.GetGameMode`)))
  (bind _output_get (set `self.Game Mode` _asbp_arkanoid_game))
  (set `/Game/Blueprints/BP_ArkanoidGame.Player Spawn Transform` (`self.GetTransform`) _output_get)
  (bind _asplayer_controller (cast `PlayerController` (`self.GetController`)))
  (set `self.Player Controller` _asplayer_controller)
  (set `SceneComponent.bAbsoluteScale` true (`self.SideLeft`))
  (set `SceneComponent.bAbsoluteScale` true (`self.SideRight`))
  (`self.Respawn`)
  (set `self.Bounds` (`.BoxExtent` (`self.GetActorBounds` false))))

(event `InputAction|LaunchBall`
  (params (Key :type "Key Structure"))
  ;[0.2159 0.006049 0.005605] Launch The Ball Input Action
  (:`Pressed`
    (if (`self.Has Powerup` "NewEnumerator2")
      (if (not (`KismetSystemLibrary.K2_IsTimerActiveHandle` (`self.Shoot Timer`)))
        (`self.Shoot`))
      (else
        (`self.Launch Ball In Paddle`)))))

(event `Key|B`
  (params (Key :type "Key Structure"))
  ;[1 1 1] Done already on arcade starter
  ;;[0.2159 0.006049 0.005605] Player Death
  (:`Pressed`
    ;;;[1 1 1] If we ran out of lives: We pause the game, show the mouse cursor, set input mode, then show game over screen.
    (set `PlayerController.bShowMouseCursor` true (`GameplayStatics.GetPlayerController` 0) :!label _label)
    (bind _returnvalue (`|CreateWidget` "/Game/Widgets/WBP_GameOverScreen.WBP_GameOverScreen_C"))
    (bind _output_get (set `self.Game Over` _returnvalue))
    (`UserWidget.AddToViewport` _output_get 0)
    (`GameplayStatics.PlaySound2D` "/Game/Sounds/Cue/sad__5__Cue.sad__5__Cue" 1.0 1.0 0.0 null null)))

(event `Die`
  ;[1 1 1] Done already on arcade starter
  ;;[0.2159 0.006049 0.005605] Player Death
  ;;;[1 1 1] Destroy All Powerups
  (bind _outactors (`GameplayStatics.GetAllActorsOfClass` "/Game/Blueprints/BP_PowerUpBase.BP_PowerUpBase_C"))
  (for _array_element _outactors
    (`self.K2_DestroyActor` _array_element))
  (`self.Remove Powerups`)
  ;;;[1 1 1] Get Rid of Particle Systems
  (`SceneComponent.SetVisibility` (`self.ParticleSystemL`) false false)
  (`SceneComponent.SetVisibility` (`self.ParticleSystemR`) false false)
  ;;;[1 1 1] Disable Input, play destroy material animation, and then Hide the Paddle.
  (`self.DisableInput` (`self.Player Controller`))
  (bind (_direction _scale) (`Timeline|Timeline_1` :!via `PlayFromStart`)
    (:`Update`
      (`KismetMaterialLibrary.SetScalarParameterValue` "/Game/Materials/Paddle/PC_Alpha.PC_Alpha" "Scale" _scale))
    (:`Finished`
      (`GameplayStatics.PlaySound2D` "/Game/Sounds/Cue/Death_Cue.Death_Cue" 1.0 1.0 0.0 null null)
      (`KismetSystemLibrary.Delay` 1.0)
      (`self.SetActorHiddenInGame` true)
      ;;;[1 1 1] Decrement Player Lives
      (`self.Add Lives` -1)
      (if (== (`/Game/Blueprints/BP_GameInstance.Lives` (`self.GameInstance`)) 0)
        ;;;[1 1 1] If we ran out of lives: We pause the game, show the mouse cursor, set input mode, then show game over screen.
        (`GameplayStatics.SetGamePaused` true)
        (goto _label)
        (else
          ;;;[1 1 1] If player still has lives: Call the Respawn Custom Event
          (`self.Respawn`))))))

(event `InputAxis|MoveRight`
  (params (AxisValue :type "Float (single-precision)"))
  ;[1 1 1] Also Done on Arcade Starter
  ;;[0.2159 0.006049 0.005605] Paddle Movement
  (if (not (or (== AxisValue 0.0) (`self.Warp Out`)))
    (`PrimitiveComponent.AddImpulse` (`self.paddle`) (`KismetMathLibrary.MakeVector` 0.0 (* AxisValue (`self.PaddleSpeed`))) "None" false)))

(event `Key|One`
  (params (Key :type "Key Structure"))
  ;[1 1 1] Done already on arcade starter
  ;;[1 1 1] Debug Cheats
  (:`Pressed`
    (`self.Add Powerup` "NewEnumerator0")))

(event `Key|G`
  (params (Key :type "Key Structure"))
  ;[1 1 1] Done already on arcade starter
  ;;[1 1 1] Debug Cheats
  (:`Pressed`
    (`/Engine/EditorBlueprintResources/StandardMacros.FlipFlop`
      (:`A`
        (`KismetSystemLibrary.ExecuteConsoleCommand` "slomo 0.1" null))
      (:`B`
        (`KismetSystemLibrary.ExecuteConsoleCommand` "slomo 1" null)))))

(event `NewBall`
  ;[1 1 1] Also Done on Arcade Starter
  ;;[0.2159 0.006049 0.005605] Make New Ball Custom Event
  (bind _returnvalue (`|SpawnActorFromClass` "/Game/Blueprints/BP_TheBall.BP_TheBall_C" (`SceneComponent.K2_GetComponentToWorld` (`self.Launch`)) "AlwaysSpawn" "OverrideRootScale" self null))
  (`self.Put Ball In Paddle` _returnvalue))

(event `Key|Two`
  (params (Key :type "Key Structure"))
  ;[1 1 1] Done already on arcade starter
  ;;[1 1 1] Debug Cheats
  (:`Pressed`
    (`self.Add Powerup` "NewEnumerator2")))

(event `Key|J`
  (params (Key :type "Key Structure"))
  ;[1 1 1] Done already on arcade starter
  ;;[1 1 1] Debug Cheats
  (:`Pressed`
    (`/Game/Blueprints/BP_TheBall.Stop` (`self.Balls`))))

(event `Key|Three`
  (params (Key :type "Key Structure"))
  ;[1 1 1] Done already on arcade starter
  ;;[1 1 1] Debug Cheats
  (:`Pressed`
    (`self.Add Powerup` "NewEnumerator3")))

(event `Respawn`
  ;[1 1 1] Done already on arcade starter
  ;;[0.2159 0.006049 0.005605] Respawn Player Paddle Custom Event
  (`self.DisableInput` (`self.Player Controller`))
  (`self.SetActorHiddenInGame` true)
  (set `self.Show Player Ready` true)
  (`GameplayStatics.PlaySound2D` "/Game/Music/Game_Start_Cue.Game_Start_Cue" 1.0 1.0 0.0 null null)
  (`KismetSystemLibrary.Delay` 2.0)
  (set `self.Show Player Ready` false)
  (`self.SetActorHiddenInGame` false)
  (`KismetMaterialLibrary.SetScalarParameterValue` "/Game/Materials/Paddle/PC_Alpha.PC_Alpha" "Scale")
  (`self.K2_SetActorTransform` (`/Game/Blueprints/BP_ArkanoidGame.Player Spawn Transform` (`self.Game Mode`)))
  (bind (_direction _alpha) (`Timeline|Timeline_0` :!via `PlayFromStart`)
    (:`Update`
      (`KismetMaterialLibrary.SetScalarParameterValue` "/Game/Materials/Paddle/PC_Alpha.PC_Alpha" "Alpha" _alpha))
    (:`Finished`
      (`self.EnableInput` (`self.Player Controller`))
      (`self.NewBall`)
      (`SceneComponent.SetVisibility` (`self.ParticleSystemL`) true false)
      (`SceneComponent.SetVisibility` (`self.ParticleSystemR`) true false))))

(event `Key|N`
  (params (Key :type "Key Structure"))
  ;[1 1 1] Done already on arcade starter
  ;;[1 1 1] Debug Cheats
  (:`Pressed`
    (`/Game/Blueprints/BP_ArkanoidGame.Add Points` (`self.Game Mode`) 500)))

(event `Key|Four`
  (params (Key :type "Key Structure"))
  ;[1 1 1] Done already on arcade starter
  ;;[1 1 1] Debug Cheats
  (:`Pressed`
    (`self.Add Powerup` "NewEnumerator4")))

(event `Key|Five`
  (params (Key :type "Key Structure"))
  ;[1 1 1] Done already on arcade starter
  ;;[1 1 1] Debug Cheats
  (:`Pressed`
    (`self.Add Powerup` "NewEnumerator5")))

(event `Key|Six`
  (params (Key :type "Key Structure"))
  ;[1 1 1] Done already on arcade starter
  ;;[1 1 1] Debug Cheats
  (:`Pressed`
    (`self.Add Powerup` "NewEnumerator8")))

(event `Put Ball In Paddle`
  (params (`New Ball In Paddle` :type "/Game/Blueprints/BP_TheBall Object Reference") (`Relative Y` :type "Float (double-precision)"))
  ;[1 1 1] Also Done on Arcade Starter
  ;;[0.2159 0.006049 0.005605] Put the ball to the paddle
  (`/Engine/EditorBlueprintResources/StandardMacros.IsValid` (`self.Ball In Paddle`)
    (:`Is Not Valid`
      (`self.Remove Ball` `New Ball In Paddle`)
      (bind _output_get (set `self.Ball In Paddle` `New Ball In Paddle`))
      (`/Game/Blueprints/BP_TheBall.Stop` _output_get)
      (`self.K2_SetActorRelativeLocation` _output_get (+ (`SceneComponent.RelativeLocation` (`self.Launch`)) (`KismetMathLibrary.MakeVector` 0.0 `Relative Y`)) false false)
      (`self.K2_AttachToActor` _output_get self "None" "KeepRelative" "SnapToTarget" "SnapToTarget" true))))

(event `Key|Seven`
  (params (Key :type "Key Structure"))
  ;[1 1 1] Done already on arcade starter
  ;;[1 1 1] Debug Cheats
  (:`Pressed`
    (`self.Add Powerup` "NewEnumerator9")))

(event `Key|Backslash`
  (params (Key :type "Key Structure"))
  ;[1 1 1] Done already on arcade starter
  ;;[1 1 1] Debug Cheats
  (:`Pressed`
    (`self.Remove Powerups` :!label _label_2)))

(event `Key|Zero`
  (params (Key :type "Key Structure"))
  ;[1 1 1] Done already on arcade starter
  ;;[1 1 1] Debug Cheats
  (:`Pressed`
    (goto _label_2)))

(fn `Add Ball`
  (params (Ball :type "/Game/Blueprints/BP_TheBall Object Reference (by ref)"))
  (`KismetArrayLibrary.Array_AddUnique` (`self.Balls`) Ball))

(fn `Add Lives`
  (params (Lives :type Integer))
  (bind _gameinstance (`self.GameInstance`))
  (if (!= Lives 0)
    (bind _output_get (set `/Game/Blueprints/BP_GameInstance.Lives` (`KismetMathLibrary.Clamp` (+ (`/Game/Blueprints/BP_GameInstance.Lives` _gameinstance) Lives) 0 (`/Game/Blueprints/BP_GameInstance.MaxLives` _gameinstance)) _gameinstance))
    (`self.On Player Lives Updated` _output_get)))

(fn `Add Powerup`
  (params (`New Powerup` :type "/Game/Blueprints/E_Powerups Enum" :default "NewEnumerator0"))
  (locals (`Remove All?` :type Boolean))
  (bind _powerup (`self.Powerup`))
  (for _array_element (`self.Get Powerups`)
    (if (`self.Compare Powerups` _array_element `New Powerup`)
      (set `local.Remove All?` true)
      (break)))
  (if (`local.Remove All?`)
    (`self.Remove Powerups`))
  (set `self.Powerup` (select `bool` (or (`|EnumEquality` `New Powerup` "NewEnumerator8") (`|EnumEquality` `New Powerup` "NewEnumerator9")) :`false` (`KismetMathLibrary.Or_IntInt` (`self.Get Bit Mask` `New Powerup`) _powerup) :`true` _powerup))
  (switch `/Game/Blueprints/E_Powerups` `New Powerup`
    (:`NewEnumerator0`
      (`GameplayStatics.PlaySound2D` "/Game/Sounds/Wav/coins__3_.coins__3_" 1.0 1.0 0.0 null null))
    (:`NewEnumerator2`
      (`self.Set Laser Mode` true)
      (`self.Launch Ball In Paddle`)
      (`SceneComponent.SetVisibility` (`self.ParticleSystemL`) false false)
      (`SceneComponent.SetVisibility` (`self.ParticleSystemR`) false false)
      (`GameplayStatics.PlaySound2D` "/Game/Sounds/Wav/retro_powerup_item_14.retro_powerup_item_14" 1.0 1.0 0.0 null null))
    (:`NewEnumerator3`
      (`self.Disrupt Ball` 3)
      (`GameplayStatics.PlaySound2D` "/Game/Sounds/Wav/item_and_powerup__13_.item_and_powerup__13_" 1.0 1.0 0.0 null null))
    (:`NewEnumerator4`
      (`self.Set Target Scale` (1.0 1.7 1.0))
      (`GameplayStatics.PlaySound2D` "/Game/Sounds/Wav/retro_boost_power_01.retro_boost_power_01" 1.0 1.0 0.0 null null)
      (`self.Launch Ball In Paddle`))
    (:`NewEnumerator5`
      (for _array_element_2 (`self.Balls`)
        (`/Game/Blueprints/BP_TheBall.Slow Ball` _array_element_2 true)
        (`GameplayStatics.PlaySound2D` "/Game/Sounds/Wav/retro_powerup_collect_08.retro_powerup_collect_08" 1.0 1.0 0.0 null null)))
    (:`NewEnumerator8`
      (`self.Add Lives` 1)
      (`GameplayStatics.PlaySound2D` "/Game/Sounds/Cue/Extra_Life_Cue.Extra_Life_Cue" 1.0 1.0 0.0 null null))
    (:`NewEnumerator9`
      (`/Game/Blueprints/BP_SidePiece.Open` (`/Game/Blueprints/BP_ArkanoidGame.Side Piece` (`self.Game Mode`)))
      (`GameplayStatics.PlaySound2D` "/Game/Sounds/Wav/item_and_powerup__11_.item_and_powerup__11_" 1.0 1.0 0.0 null null))))

(fn `Bogus`)

(fn `Compare Powerups`
  (params (`Current Powerup` :type "/Game/Blueprints/E_Powerups Enum" :default "NewEnumerator0") (`New Powerup` :type "/Game/Blueprints/E_Powerups Enum" :default "NewEnumerator0"))
  (returns (`Remove?` :type Boolean))
  (return (not (or (and (`|EnumEquality` `Current Powerup` "NewEnumerator0") (`|EnumEquality` `New Powerup` "NewEnumerator5")) (and (`|EnumEquality` `Current Powerup` "NewEnumerator3") (`|EnumEquality` `New Powerup` "NewEnumerator5")) (and (`|EnumEquality` `Current Powerup` "NewEnumerator5") (or (`|EnumEquality` `New Powerup` "NewEnumerator0") (`|EnumEquality` `New Powerup` "NewEnumerator3"))) (`|EnumEquality` `New Powerup` "NewEnumerator8")))))

(fn `Disrupt Ball`
  (params (`Max Balls` :type Integer :default 3))
  (locals (`Top Most Ball` :type "/Game/Blueprints/BP_TheBall Object Reference") (`Max Ball Index` :type Integer))
  (bind _top_most_ball (`local.Top Most Ball`))
  (bind _output_get (set `local.Top Most Ball` (`self.Get Top Most Ball`)))
  (`/Engine/EditorBlueprintResources/StandardMacros.IsValid` _output_get
    (:`Is Valid`
      (bind _output_get_2 (set `local.Max Ball Index` (- (- `Max Balls` (`KismetArrayLibrary.Array_Length` (`self.Balls`))) 1)))
      (for _ (range (+ _output_get_2 1))
        (bind _returnvalue (`|SpawnActorFromClass` "/Game/Blueprints/BP_TheBall.BP_TheBall_C" (`self.GetTransform` _top_most_ball) "AlwaysSpawn" "OverrideRootScale" self null))
        (`/Game/Blueprints/BP_TheBall.Launch` _returnvalue (`KismetMathLibrary.Conv_RotatorToVector` (`KismetMathLibrary.TransformRotation` (`self.GetTransform` _top_most_ball) (`KismetMathLibrary.MakeRotator` 0.0 0.0 (`KismetMathLibrary.RandomFloatInRange` -180.0 180.0)))))))
    (:`Is Not Valid`
      (`KismetSystemLibrary.PrintString` "No Top Most Ball Found" true true (struct :`R` 1.0 :`A` 1.0)))))

(fn `Get Bit Mask`
  (params (Powerup :type "/Game/Blueprints/E_Powerups Enum" :default "NewEnumerator0"))
  (returns (`Bit Mask` :type Integer))
  (return (select `/Game/Blueprints/E_Powerups` Powerup :`NewEnumerator0` 1 :`NewEnumerator2` 2 :`NewEnumerator3` 4 :`NewEnumerator4` 8 :`NewEnumerator5` 16 :`NewEnumerator8` 32 :`NewEnumerator9` 64)))

(fn `Get Hit Angle`
  (params (`Hit Component` :type "PrimitiveComponent Object Reference"))
  (returns (Angle :type "Float (double-precision)"))
  (locals (`Return Angle` :type "Float (double-precision)" :default 45.0))
  (if (== `Hit Component` (`self.paddle`))
    (set `local.Return Angle` 5.0)
    (elif (or (== `Hit Component` (`self.SideRight`)) (== `Hit Component` (`self.SideLeft`)))
      (set `local.Return Angle` 45.0)))
  (return (`local.Return Angle`)))

(fn `Get Powerups`
  (returns (Powerups :type "Array of /Game/Blueprints/E_Powerups Enum"))
  (locals (`Powerup List` :type "Array of /Game/Blueprints/E_Powerups Enum"))
  (for _index (range (enumcount `/Game/Blueprints/E_Powerups`))
    (bind _returnvalue (cast `/Game/Blueprints/E_Powerups` (`KismetMathLibrary.Conv_IntToByte` _index)))
    (if (`self.Has Powerup` _returnvalue)
      (`KismetArrayLibrary.Array_Add` (`local.Powerup List`) _returnvalue)))
  (return (`local.Powerup List`)))

(fn `Get Top Most Ball`
  (returns (`Top Most Ball` :type "/Game/Blueprints/BP_TheBall Object Reference"))
  (locals (`Best Ball` :type "/Game/Blueprints/BP_TheBall Object Reference"))
  (bind _best_ball (`local.Best Ball`))
  (bind _returnvalue_x (`KismetMathLibrary.BreakVector` (`self.K2_GetActorLocation` _best_ball)))
  (for _array_element (`self.Balls`)
    (`/Engine/EditorBlueprintResources/StandardMacros.IsValid` _best_ball
      (:`Is Valid`
        (bind _returnvalue_x_2 (`KismetMathLibrary.BreakVector` (`self.K2_GetActorLocation` _array_element)))
        (if (> _returnvalue_x_2 _returnvalue_x)
          (set `local.Best Ball` _array_element :!label _label)))
      (:`Is Not Valid`
        (goto _label))))
  (return _best_ball))

(fn `Has Powerup`
  (params (Powerup :type "/Game/Blueprints/E_Powerups Enum" :default "NewEnumerator0"))
  (returns (Result :type Boolean))
  (return (!= (`KismetMathLibrary.And_IntInt` (`self.Get Bit Mask` Powerup) (`self.Powerup`)) 0)))

(fn `Launch Ball In Paddle`
  (bind _ball_in_paddle (`self.Ball In Paddle`))
  (`/Engine/EditorBlueprintResources/StandardMacros.IsValid` _ball_in_paddle
    (:`Is Valid`
      (`/Game/Blueprints/BP_TheBall.Launch` _ball_in_paddle (* (- (`self.GetActorForwardVector`) (`KismetMathLibrary.Normal` (`self.GetVelocity`))) (1.0 -1.0 1.0)))
      (set `self.Ball In Paddle` null)
      (`GameplayStatics.PlaySound2D` "/Game/Sounds/Cue/Hit_Paddle_Cue.Hit_Paddle_Cue" 1.0 1.0 0.0 null null))))

(fn `Remove Ball`
  (params (Ball :type "/Game/Blueprints/BP_TheBall Object Reference (by ref)") (`Check Death` :type Boolean))
  (bind _balls (`self.Balls`))
  (bind _returnvalue (`KismetArrayLibrary.Array_RemoveItem` _balls Ball))
  (if (and _returnvalue (== (`KismetArrayLibrary.Array_Length` _balls) 0) `Check Death`)
    (`self.Die`)))

(fn `Remove Powerups`
  (locals (`Top Most Ball` :type "/Game/Blueprints/BP_TheBall Object Reference"))
  (`|ExecutionSequence`
    (:`then_0`
      (`self.Has Powerup Macro` "NewEnumerator2"
        (:`True`
          (`self.Set Laser Mode` false))))
    (:`then_1`
      (`self.Has Powerup Macro` "NewEnumerator3"
        (:`True`
          (set `local.Top Most Ball` (`self.Get Top Most Ball`))
          (bind (_arrayindex _arrayelement) (`/Engine/EditorBlueprintResources/StandardMacros.ReverseForEachLoop` (`self.Balls`))
            (:`LoopBody`
              (if (!= _arrayelement (`local.Top Most Ball`))
                (`self.K2_DestroyActor` _arrayelement)))))))
    (:`then_2`
      (`self.Has Powerup Macro` "NewEnumerator4"
        (:`True`
          (`self.Set Target Scale` (1.0 1.0 1.0)))))
    (:`then_3`
      (`self.Has Powerup Macro` "NewEnumerator5"
        (:`True`
          (for _array_element (`self.Balls`)
            (`/Game/Blueprints/BP_TheBall.Slow Ball` _array_element false)))))
    (:`then_4`
      (set `self.Powerup` 0))))

(fn `Set Laser Mode`
  (params (`Laser Mode` :type Boolean))
  (bind _returnvalue (select `bool` `Laser Mode` :`false` "/Game/Meshes/corner.corner" :`true` "/Game/Meshes/LaserEnd.LaserEnd" :!type "StaticMesh Object Reference"))
  (`StaticMeshComponent.SetStaticMesh` (`self.SideRight`) _returnvalue)
  (`StaticMeshComponent.SetStaticMesh` (`self.SideLeft`) _returnvalue))

(fn `Set Target Scale`
  (params (`Target Scale` :type "Vector Structure"))
  (set `self.Target Scale` `Target Scale`)
  (`self.SetActorTickEnabled` true))

(fn `Shoot`
  (bind _returnvalue (`KismetSystemLibrary.K2_SetTimer` self "BOGUS" (`self.Shoot Rate`)))
  (set `self.Shoot Timer` _returnvalue)
  (for _array_element (`|MakeArray` (`self.SideRight`) (`self.SideLeft`))
    (bind (_returnvalue_location _returnvalue_rotation _returnvalue_scale) (`KismetMathLibrary.BreakTransform` (`SceneComponent.K2_GetComponentToWorld` _array_element)))
    (`|SpawnActorFromClass` "/Game/Blueprints/BP_Projectile.BP_Projectile_C" (`KismetMathLibrary.MakeTransform` _returnvalue_location (struct) _returnvalue_scale) "AlwaysSpawn" "OverrideRootScale" null null)
    (`GameplayStatics.PlaySound2D` "/Game/Sounds/Cue/retro_laser_gun_shoot_53_Cue.retro_laser_gun_shoot_53_Cue" 1.0 1.0 0.0 null null)))

(fn `UserConstructionScript`)

(fn `Warp`
  (bind _ball_in_paddle (`self.Ball In Paddle`))
  (`PrimitiveComponent.SetCollisionResponseToChannel` (`self.paddle`) "ECC_WorldStatic" "ECR_Ignore")
  (`PrimitiveComponent.SetCollisionResponseToChannel` (`self.SideRight`) "ECC_WorldStatic" "ECR_Ignore")
  (`PrimitiveComponent.SetCollisionResponseToChannel` (`self.SideLeft`) "ECC_WorldStatic" "ECR_Ignore")
  (`PrimitiveComponent.SetCollisionResponseToChannel` (`self.Box`) "ECC_WorldStatic" "ECR_Ignore")
  (`self.DisableInput` (`GameplayStatics.GetPlayerController` 0))
  (`/Game/Blueprints/BP_TheBall.Stop` (`self.Balls`))
  (`SceneComponent.SetVisibility` (`self.ParticleSystemL`) false false)
  (`SceneComponent.SetVisibility` (`self.ParticleSystemR`) false false)
  (set `self.Warp Out` true)
  (`self.SetActorTickEnabled` true)
  (`/Engine/EditorBlueprintResources/StandardMacros.IsValid` _ball_in_paddle
    (:`Is Valid`
      (`self.SetActorEnableCollision` _ball_in_paddle false))))