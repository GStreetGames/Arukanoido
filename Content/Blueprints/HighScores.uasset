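; High score table logic that finds where a new score ranks and inserts it into the Entries list.
; GetHighScoreIndex returns the index of the first entry whose score the new score meets or beats, so ties rank above existing entries.
; CreateHighScoreEntryAtIndex inserts an unnamed entry with round and score at a valid index, then removes index 10 to cap the table at ten.
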(fn `Create High Score Entry at Index`
  (params (Round :type String) (Score :type Integer) (Index :type Integer))
  (bind _entries (`self.Entries`))
  (if (`KismetArrayLibrary.Array_IsValidIndex` (`self.Entries`) Index)
    (`KismetArrayLibrary.Array_Insert` _entries (make `/Game/Blueprints/S_HighScoreEntry` "" Round Score) Index)
    (`KismetArrayLibrary.Array_Remove` _entries 10)))

(fn `Get High Score Index`
  (params (Score :type Integer))
  (returns (Index :type Integer))
  (locals (`High Score Index` :type Integer :default -1))
  (for (_array_element _array_index) (`self.Entries`)
    (if (>= Score (`.Score_8_CB784F9D45510F242CD717B7CA916CAA` (break `/Game/Blueprints/S_HighScoreEntry` _array_element)))
      (set `local.High Score Index` _array_index)
      (break)))
  (return (`local.High Score Index`)))