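; BP_TheBall is the physics-driven ball of an Arkanoid game, registering with its owning player on launch and deregistering on destruction.
; Launch applies a planar impulse, and each hit updates the reflected Direction and takes an angle from the paddle when struck.
; Velocity is then speed-clamped and its yaw snapped to angle-based steps in a slightly randomized rotated frame.
; SlowBall pins speed to the minimum while active.
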(event `self.ReceiveBeginPlay`
  ;[0.0892 1 0.02729] Cast To The Player Base and the Game Mode on Begin Play! Then Store them as variables.
  (bind _asbp_arkanoid_player_base (cast `/Game/Blueprints/BP_ArkanoidPlayerBase` (`self.GetOwner`)))
  (set `self.PlayerBase` _asbp_arkanoid_player_base)
  (bind _asbp_arkanoid_game (cast `/Game/Blueprints/BP_ArkanoidGame` (`GameplayStatics.GetGameMode`)))
  (set `self.GameMode` _asbp_arkanoid_game)
  (set `SceneComponent.bAbsoluteScale` true (`self.BallMesh`)))

(event `self.ReceiveDestroyed`
  ;[0.2159 0.006049 0.005605] On Ball Death, remove the ball on the player
  (`/Game/Blueprints/BP_ArkanoidPlayerBase.Remove Ball` (`self.PlayerBase`) self true))

(event `Stop`
  ;[0.9635 0.01546 0] STOP The ball
  (`PrimitiveComponent.SetSimulatePhysics` (`self.BallMesh`) false))

(event `self.ReceiveHit`
  (params (MyComp :type "PrimitiveComponent Object Reference") (Other :type "Actor Object Reference") (OtherComp :type "PrimitiveComponent Object Reference") (bSelfMoved :type Boolean) (HitLocation :type "Vector Structure") (HitNormal :type "Vector Structure") (NormalImpulse :type "Vector Structure") (Hit :type "HitResult Structure (by ref)"))
  ;[0.2159 0.006049 0.005605] On Hit
  (`self.Process Hit` Hit))

(event `Launch`
  (params (Direction :type "Vector Structure"))
  (bind _ballmesh (`self.BallMesh`))
  ;[0.2159 0.006049 0.005605] Add Impulse to Direction Based on Speed
  (bind _output_get (set `self.Direction` Direction))
  (`PrimitiveComponent.SetSimulatePhysics` _ballmesh true)
  (`PrimitiveComponent.AddImpulse` _ballmesh (* (* _output_get (`self.Min Speed`)) (1.0 1.0 0.0)) "None" true)
  (`/Game/Blueprints/BP_ArkanoidPlayerBase.Add Ball` (`self.PlayerBase`) self))

(fn `Clamp Velocity`
  (bind _returnvalue (`PrimitiveComponent.GetPhysicsLinearVelocity` (`self.BallMesh`) "None"))
  (`PrimitiveComponent.SetPhysicsLinearVelocity` (`self.BallMesh`) (`KismetMathLibrary.ClampVectorSize` _returnvalue (`self.Min Speed`) (select `bool` (`self.Is Slowed`) :`false` (`self.Max Speed`) :`true` (`self.Min Speed`))) false "None"))

(fn `ClampAngleAndVelocity`
  (params (Angle :type "Float (double-precision)"))
  (bind _returnvalue (* Angle 2.0))
  (bind _returnvalue_2 (`KismetMathLibrary.MakeRotator` 0.0 0.0 (+ Angle (`KismetMathLibrary.RandomFloatInRange` 1.0 5.0))))
  ;[1 1 1] Vector Math Calculation to Clamp Angles and speed. Clamps angles to only 0, 90, 180, and their respective minus values.
  (bind _returnvalue_3 (`PrimitiveComponent.GetPhysicsLinearVelocity` (`self.BallMesh`) "None"))
  (bind _returnvalue_4 (`KismetMathLibrary.ClampVectorSize` _returnvalue_3 (`self.Min Speed`) (`self.Max Speed`)))
  (bind (_returnvalue_roll _returnvalue_pitch _returnvalue_yaw) (`KismetMathLibrary.BreakRotator` (`KismetMathLibrary.MakeRotFromX` (`KismetMathLibrary.GreaterGreater_VectorRotator` _returnvalue_4 _returnvalue_2))))
  ;[0.6222 1 0.5625] Function Setup (the easy part)
  (`PrimitiveComponent.SetPhysicsLinearVelocity` (`self.BallMesh`) (* (`KismetMathLibrary.LessLess_VectorRotator` (`KismetMathLibrary.Conv_RotatorToVector` (`KismetMathLibrary.MakeRotator` 0.0 0.0 (`KismetMathLibrary.Conv_IntToDouble` (* (`KismetMathLibrary.Round` (/ _returnvalue_yaw _returnvalue)) (`KismetMathLibrary.FTrunc` _returnvalue))))) _returnvalue_2) (`KismetMathLibrary.VSize` _returnvalue_4)) false "None"))

(fn `Process Hit`
  (params (Hit :type "HitResult Structure (by ref)"))
  (locals (Angle :type "Float (double-precision)" :default 45.0))
  (bind (_bblockinghit _binitialoverlap _time _distance _location _impactpoint _normal _impactnormal _physmat _hitactor _hitcomponent) (`GameplayStatics.BreakHitResult` Hit))
  ;[1 1 1] Calculate Hit Vector, Set Direction, then Clamp the Angle and Velocity
  (set `self.Direction` (`KismetMathLibrary.GetReflectionVector` (`self.Direction`) _impactnormal))
  (bind _asbp_arkanoid_player_base (cast `/Game/Blueprints/BP_ArkanoidPlayerBase` _hitactor)
    (:`then`
      (set `local.Angle` (`/Game/Blueprints/BP_ArkanoidPlayerBase.Get Hit Angle` _asbp_arkanoid_player_base _hitcomponent)))
    (:`CastFailed`
      _))
  (`self.ClampAngleAndVelocity` (`local.Angle`)))

(fn `Slow Ball`
  (params (Slow :type Boolean))
  (set `self.Is Slowed` Slow)
  (`self.Clamp Velocity`))

(fn `UserConstructionScript`)