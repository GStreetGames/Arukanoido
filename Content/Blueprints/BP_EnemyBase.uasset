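; Base enemy for the Arkanoid game that drifts erratically, awards points and dies when touched by the paddle, ball or a projectile.
; Tick applies constant X force plus a sideways force, whose direction a self-resetting timer re-rolls at random intervals.
; Hits by the ball also knock it away with a radial impulse.
; It registers with the game mode on BeginPlay, and on destruction unregisters with explosion and sound.
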(event `self.ReceiveTick`
  (params (DeltaSeconds :type "Float (single-precision)"))
  ;[1 1 1] Random retard movement
  (`PrimitiveComponent.AddForce` (`self.EnemyMesh`) (`KismetMathLibrary.MakeVector` -14.119999 (`self.Side Force`)) "None" true))

(event `Randomize Side Force`
  ;[1 1 1] Random retard movement
  (set `self.Side Force` (select `bool` (`KismetMathLibrary.RandomBool`) :`false` -132.050003 :`true` 143.869995 :!type "Float (single-precision)"))
  (`KismetSystemLibrary.K2_SetTimerDelegate` (delegate `Randomize Side Force`) (`KismetMathLibrary.RandomFloatInRange` 0.26 1.65) true))

(event `self.ReceiveDestroyed`
  ;[1 1 1] Destruction Event
  (`/Game/Blueprints/BP_ArkanoidGame.Remove Enemy` (`self.Game Mode`))
  (`GameplayStatics.SpawnEmitterAtLocation` "/Game/ExampleContent/Blueprint_Communication/Effects/P_Explosion_Bomb.P_Explosion_Bomb" (`self.K2_GetActorLocation`))
  (`GameplayStatics.PlaySound2D` (`self.SoundEffect`) 1.0 1.0 0.0 null null))

(event `self.ReceiveActorBeginOverlap`
  (params (OtherActor :type "Actor Object Reference"))
  ;[1 1 1] On Hit, Process destruction and award points to the player if the ball, laser, or paddle, touches the enemy.
  (`self.Handle Damage` OtherActor))

(event `self.ReceiveHit`
  (params (MyComp :type "PrimitiveComponent Object Reference") (Other :type "Actor Object Reference") (OtherComp :type "PrimitiveComponent Object Reference") (bSelfMoved :type Boolean) (HitLocation :type "Vector Structure") (HitNormal :type "Vector Structure") (NormalImpulse :type "Vector Structure") (Hit :type "HitResult Structure (by ref)"))
  ;[1 1 1] On Hit, Process destruction and award points to the player if the ball, laser, or paddle, touches the enemy.
  (bind _asbp_the_ball (cast `/Game/Blueprints/BP_TheBall` Other))
  (`PrimitiveComponent.AddRadialImpulse` (`/Game/Blueprints/BP_TheBall.BallMesh` _asbp_the_ball) (`self.K2_GetActorLocation`) 1777.0 3700.0 "RIF_Constant" true)
  (`self.Handle Damage` Other))

(event `self.ReceiveBeginPlay`
  ;[1 1 1] Begin Play
  (bind _asbp_arkanoid_game (cast `/Game/Blueprints/BP_ArkanoidGame` (`GameplayStatics.GetGameMode`)))
  (bind _output_get (set `self.Game Mode` _asbp_arkanoid_game))
  (`/Game/Blueprints/BP_ArkanoidGame.Add Enemy` _output_get)
  (`self.Randomize Side Force`))

(event `Handle Damage`
  (params (OtherActor :type "Actor Object Reference"))
  ;[1 1 1] Handle Damage Function
  (if (or (`.bSuccess` (cast `/Game/Blueprints/BP_ArkanoidPlayerBase` OtherActor :!pure true)) (`.bSuccess` (cast `/Game/Blueprints/BP_Projectile` OtherActor :!pure true)) (`.bSuccess` (cast `/Game/Blueprints/BP_TheBall` OtherActor :!pure true)))
    (`/Game/Blueprints/BP_ArkanoidGame.Add Points` (`self.Game Mode`) (`self.EnemyPoints`))
    (`self.K2_DestroyActor`)))

(fn `UserConstructionScript`)