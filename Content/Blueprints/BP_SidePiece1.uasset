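; BP_SidePiece1 is a level piece that visually opens through its material and then enables a warp trigger.
; BeginPlay creates a dynamic material instance, and Open plays the OpenClose timeline to drive its "Open" scalar.
; When the timeline finishes, WarpTrigger gets query-only collision.
; IsMoving blocks replays and is never reset here; both trigger overlap handlers are empty.
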(event `Open`
  (if (not (`self.Is Moving`))
    (bind (_direction _alpha) (`Timeline|Open / Close` :!via `PlayFromStart`)
      (:`Update`
        (`MaterialInstanceDynamic.SetScalarParameterValue` (`self.Material Instance`) "Open" _alpha)
        (set `self.Is Moving` true))
      (:`Finished`
        (`PrimitiveComponent.SetCollisionEnabled` (`self.Warp Trigger`) "QueryOnly")))))

(event `self.Warp Trigger.OnComponentBeginOverlap`
  (params (OverlappedComponent :type "PrimitiveComponent Object Reference") (OtherActor :type "Actor Object Reference") (OtherComp :type "PrimitiveComponent Object Reference") (OtherBodyIndex :type Integer) (bFromSweep :type Boolean) (SweepResult :type "HitResult Structure (by ref)")))

(event `self.Level Clear Trigger.OnComponentBeginOverlap`
  (params (OverlappedComponent :type "PrimitiveComponent Object Reference") (OtherActor :type "Actor Object Reference") (OtherComp :type "PrimitiveComponent Object Reference") (OtherBodyIndex :type Integer) (bFromSweep :type Boolean) (SweepResult :type "HitResult Structure (by ref)")))

(event `self.ReceiveBeginPlay`
  (bind _staticmeshcomponent (`self.StaticMeshComponent`))
  (bind _returnvalue (`PrimitiveComponent.CreateDynamicMaterialInstance` _staticmeshcomponent 0 (`PrimitiveComponent.GetMaterial` _staticmeshcomponent 0) "None"))
  (set `self.Material Instance` _returnvalue))

(fn `UserConstructionScript`)