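; BP_TopPiece is a top piece in an Arkanoid game that registers with BP_ArkanoidGame and acts as a spawn hatch for enemies.
; Spawn calls queue enemies and start opening if the piece is idle.
; A timeline animates opening and closing through a dynamic material's "Open" parameter.
; Once fully open it spawns an enemy and closes, then reopens while any remain queued.
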(event `Spawn`
  ;[1 1 1] Custom Spawn Function called
  (`/Engine/EditorBlueprintResources/StandardMacros.IncrementInt` (`self.Enemies to Spawn`)
    (:`  `
      (if (not (`self.Is Moving?`))
        (`self.Open`)))))

(event `Open`
  (bind _returnvalue_location (`KismetMathLibrary.BreakTransform` (`self.GetTransform`)))
  ;[1 1 1] Open and Close Animation done with material...
  (bind (_direction _alpha) (`Timeline|Open / Close` :!via `PlayFromStart` :!label _label)
    (:`Update`
      (`MaterialInstanceDynamic.SetScalarParameterValue` (`self.Material Instance`) "Open" _alpha)
      (set `self.Is Moving?` true))
    (:`Finished`
      (set `self.Is Moving?` false)
      (if (== _alpha 1.0)
        (`|SpawnActorFromClass` (`self.Enemy Class`) (`KismetMathLibrary.MakeTransform` (- _returnvalue_location (250.0 0.0 -50.0)) (struct :`Pitch` -90.0) (0.7 0.7 0.7)) "AlwaysSpawn" "OverrideRootScale" null null)
        (`/Engine/EditorBlueprintResources/StandardMacros.DecrementInt` (`self.Enemies to Spawn`)
          (:`  `
            (`self.Close`)))
        (elif (> (`self.Enemies to Spawn`) 0)
          (`self.Open`))))))

(event `Close`
  ;[1 1 1] Open and Close Animation done with material...
  (goto _label :!via `ReverseFromEnd`))

(event `self.ReceiveBeginPlay`
  (bind _staticmeshcomponent (`self.StaticMeshComponent`))
  ;[1 1 1] Event Begin Play - set up top pieces and the dynamic material.
  (bind _asbp_arkanoid_game (cast `/Game/Blueprints/BP_ArkanoidGame` (`GameplayStatics.GetGameMode`)))
  (`/Game/Blueprints/BP_ArkanoidGame.Add Top Piece` _asbp_arkanoid_game self)
  (bind _returnvalue (`PrimitiveComponent.CreateDynamicMaterialInstance` _staticmeshcomponent 0 (`PrimitiveComponent.GetMaterial` _staticmeshcomponent 0) "None"))
  (set `self.Material Instance` _returnvalue))

(fn `UserConstructionScript`)