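; Game mode for an Arkanoid game that manages score, enemies, block count and level progression.
; On login it derives the current level from the map name; on BeginPlay it creates the HUD and, after a random delay, spawns enemies from random registered top pieces, replacing each one removed.
; Points persist in the game instance, update listeners and award extra lives at score intervals.
; Clearing all blocks opens the next numbered level, with wraparound.
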(event `self.ReceiveBeginPlay`
  ;[0.162 0.006512 0.006512] Begin Play, cast then set Player Base, then count all blocks by using the Tag you gave the base block class.
  (bind _asbparkanoid_player_controller (cast `/Game/Blueprints/BPArkanoidPlayerController` (`GameplayStatics.GetPlayerController` 0)))
  (set `self.PlayerController` _asbparkanoid_player_controller)
  (bind _asbp_arkanoid_player_base (cast `/Game/Blueprints/BP_ArkanoidPlayerBase` (`GameplayStatics.GetPlayerPawn` 0)))
  (set `self.Player Base` _asbp_arkanoid_player_base)
  (bind _returnvalue (`|CreateWidget` "/Game/Widgets/WBP_ArkanoidHUDWidget.WBP_ArkanoidHUDWidget_C"))
  (bind _output_get (set `self.HUDWidget` _returnvalue))
  (`UserWidget.AddToViewport` _output_get 0)
  (`self.On Points Updated` (`/Game/Blueprints/BP_GameInstance.PlayerPoints` (`self.GameInstance`)))
  ;[1 1 1] Delay and enemy spawn
  (`KismetSystemLibrary.Delay` (`KismetMathLibrary.RandomFloatInRange` 1.0 7.0))
  (for _ (range 1 (+ (`self.Max Enemy Count`) 1))
    (`self.Spawn Enemy`)))

(event `self.K2_PostLogin`
  (params (NewPlayer :type "PlayerController Object Reference"))
  ;[1 1 1] Event Post Login
  (bind _asbp_game_instance (cast `/Game/Blueprints/BP_GameInstance` (`GameplayStatics.GetGameInstance`)))
  (set `self.GameInstance` _asbp_game_instance)
  (bind _returnvalue (`GameplayStatics.GetCurrentLevelName` true))
  (bind _output_get (set `self.Round` (`KismetStringLibrary.RightChop` _returnvalue 5)))
  (set `/Game/Blueprints/BP_GameInstance.CurrentLevel` (`KismetStringLibrary.Conv_StringToInt` _output_get) (`self.GameInstance`)))

(event `Add Top Piece`
  (params (`Top Piece` :type "/Game/Blueprints/BP_TopPiece Object Reference (by ref)"))
  ;[1 1 1] Block and enemy custom events
  (`KismetArrayLibrary.Array_Add` (`self.Top Pieces`) `Top Piece`))

(event `Add Enemy`
  ;[1 1 1] Block and enemy custom events
  (`/Engine/EditorBlueprintResources/StandardMacros.IncrementInt` (`self.Enemy Count`)))

(event `UnpauseEvent`
  (bind _playercontroller (`self.PlayerController`))
  ;[1 1 1] Unpause custom event
  (`GameplayStatics.SetGamePaused` false)
  (set `PlayerController.bShowMouseCursor` false _playercontroller)
  (`WidgetBlueprintLibrary.SetInputMode_GameOnly` _playercontroller)
  (`Widget.SetVisibility` (`/Game/Widgets/WBP_ArkanoidHUDWidget.WBP_PauseMenu` (`self.HUDWidget`)) "Hidden"))

(event `Remove Enemy`
  ;[1 1 1] Block and enemy custom events
  (`/Engine/EditorBlueprintResources/StandardMacros.DecrementInt` (`self.Enemy Count`)
    (:`  `
      (`self.Spawn Enemy`))))

(event `Add to Remaning Blocks`
  ;[1 1 1] Block and enemy custom events
  (`/Engine/EditorBlueprintResources/StandardMacros.IncrementInt` (`self.Block Remaining`)))

(event `Subtract from Remaining Blocks`
  ;[1 1 1] Block and enemy custom events
  (bind _result (`/Engine/EditorBlueprintResources/StandardMacros.DecrementInt` (`self.Block Remaining`))
    (:`  `
      (if (<= _result 0)
        (`self.Level Clear`)
        (else
          (`/Engine/EditorBlueprintResources/StandardMacros.IncrementInt` (`self.Powerup Block Counter`)))))))

(event `Level Clear`
  ;[1 1 1] Level Cleared Action Logic
  (`self.IncrementLevel`)
  (`GameplayStatics.OpenLevel` (`KismetStringLibrary.Conv_StringToName` (`KismetStringLibrary.Concat_StrStr` "Level" (`KismetStringLibrary.Conv_IntToString` (`/Game/Blueprints/BP_GameInstance.CurrentLevel` (`self.GameInstance`)))))))

(fn `Add Points`
  (params (Points :type Integer))
  (locals (`Number of Lives To Add` :type Integer :default 0))
  (bind _gameinstance (`self.GameInstance`))
  (if (!= Points 0)
    (bind _output_get (set `/Game/Blueprints/BP_GameInstance.PlayerPoints` (+ (`/Game/Blueprints/BP_GameInstance.PlayerPoints` _gameinstance) Points) _gameinstance))
    (`self.On Points Updated` _output_get)
    (bind _output_get_2 (set `local.Number of Lives To Add` (/ (- _output_get (`self.Last Extra Life Player Points`)) (`self.Extra Life Points`))))
    (if (> _output_get_2 0)
      (`/Game/Blueprints/BP_ArkanoidPlayerBase.Add Lives` (`self.Player Base`) _output_get_2)
      (set `self.Last Extra Life Player Points` (+ (`self.Last Extra Life Player Points`) (* _output_get_2 (`self.Extra Life Points`)))))))

(fn `IncrementLevel`
  (locals (Level1 :type Integer :default 1))
  (bind _gameinstance (`self.GameInstance`))
  (bind _currentlevel (`/Game/Blueprints/BP_GameInstance.CurrentLevel` _gameinstance))
  (bind _result (`/Engine/EditorBlueprintResources/StandardMacros.IncrementInt` _currentlevel)
    (:`  `
      (bind _output_get (set `/Game/Blueprints/BP_GameInstance.CurrentLevel` (select `bool` (== _currentlevel 4) :`false` _result :`true` (`local.Level1`)) _gameinstance))
      (`self.OnUpdateLevel` _output_get))))

(fn `Spawn Enemy`
  (bind _top_pieces (`self.Top Pieces`))
  (`/Game/Blueprints/BP_TopPiece.Spawn` (`|GetArrayItem` _top_pieces (`KismetMathLibrary.RandomIntegerInRange` 0 (- (`KismetArrayLibrary.Array_Length` _top_pieces) 1)))))

(fn `UserConstructionScript`)